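; ItemDataComponent is an actor component that makes its owning actor a pickup for the inventory system.
; On BeginPlay it sets the owner to replicate.
; Its Interactwith event passes the item's row name and quantity to the interacting player's InventorySystem and destroys the owner if the add succeeds.
; LookAt returns an empty string.
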(event EventBeginPlay
  (Networking|SetReplicates (Components|GetOwner) true))

(event EventTick
  (params (DeltaSeconds :type Float%20%28single-precision%29)))

(event EventInteractwith
  (params (PlayerCharacter :type My%20First%20Person%20Character%20Object%20Reference))
  (bind _inventorysystem (Variables|/Game/MyContent/Blueprints/Characters/MyFirstPersonCharacter.MyFirstPersonCharacter_C|GetInventorySystem PlayerCharacter))
  (Utilities|IsValid _inventorysystem
    (:Is%20Valid
      (bind _success (Default|AddtoInventory _inventorysystem (.rowname (Variables|Default|GetItemID)) (Variables|Default|GetQuantity)))
      (if _success
        (Actor|DestroyActor (Components|GetOwner))))))

(fn Lookat
  (return ""))